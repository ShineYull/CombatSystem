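; NPC combat component that gives its owner directional hit reactions and melee impact effects.
; RecieveDamage classifies the attacker's relative yaw into four directions and passes it to ServerPlayHitAnimation.
; That event plays the matching hit montage on the Character mesh, then calls MultiPlayMontage with it, apparently for replication.
; Separately, CallSpawnHitFX spawns a particle aligned to the impact normal and a quiet sword-hit sound at the owner.
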(event `/Game/CombatSystem/Blueprint/Component/BI_CombatGeneral.CallSpawnHitFX`
  (params (InImpactNormal :type "Vector Structure"))
  (`self.SpawnMeleeEffects` InImpactNormal))

(event `ServerPlayHitAnimation`
  (params (InHitFromDirection :type "/Game/CombatSystem/Blueprint/Component/Misc/GeneralEnums/E_CardinalDirection Enum" :default "NewEnumerator0"))
  (bind _returnvalue (select `/Game/CombatSystem/Blueprint/Component/Misc/GeneralEnums/E_CardinalDirection` InHitFromDirection :`NewEnumerator1` "/Game/CombatSystem/Art/Anim/Sword/HitReact/AM_Hit_01_F.AM_Hit_01_F" :`NewEnumerator2` "/Game/CombatSystem/Art/Anim/Sword/HitReact/AM_Hit_01_B.AM_Hit_01_B" :`NewEnumerator3` "/Game/CombatSystem/Art/Anim/Sword/HitReact/AM_Hit_01_L.AM_Hit_01_L" :`NewEnumerator4` "/Game/CombatSystem/Art/Anim/Sword/HitReact/AM_Hit_01_R.AM_Hit_01_R" :!type "AnimMontage Object Reference"))
  (bind _ascharacter (cast `Character` (`self.GetOwner`)))
  (bind _mesh (`Character.Mesh` _ascharacter))
  (`|PlayMontage` _mesh _returnvalue
    (:`then`
      (`self.MultiPlayMontage` _mesh _returnvalue))))

(event `MultiPlayMontage`
  (params (InSkeletalMeshComponent :type "SkeletalMeshComponent Object Reference") (MontageToPlay :type "AnimMontage Object Reference"))
  (`|PlayMontage` InSkeletalMeshComponent MontageToPlay))

(fn `GetHitDirection`
  (params (InAttackingActor :type "Actor Object Reference"))
  (returns (OutDirection :type "/Game/CombatSystem/Blueprint/Component/Misc/GeneralEnums/E_CardinalDirection Enum"))
  (locals (Local_NormalizedYaw :type "Float (double-precision)"))
  (bind _local_normalizedyaw (`local.Local_NormalizedYaw`))
  (bind _local_normalizedyaw_2 (`local.Local_NormalizedYaw`))
  (bind _local_normalizedyaw_3 (`local.Local_NormalizedYaw`))
  (bind (_returnvalue_roll _returnvalue_pitch _returnvalue_yaw) (`KismetMathLibrary.BreakRotator` (`KismetMathLibrary.NormalizedDeltaRotator` (`Actor.K2_GetActorRotation` (`self.GetOwner`)) (`KismetMathLibrary.FindLookAtRotation` (`Actor.GetActorEyesViewPoint` (`self.GetOwner`)) (`Actor.K2_GetActorLocation` (`local.InAttackingActor`))))))
  (set `local.Local_NormalizedYaw` _returnvalue_yaw)
  (if (and (>= _local_normalizedyaw_2 -45.0) (<= _local_normalizedyaw_2 45.0))
    (return "NewEnumerator1")
    (elif (and (> _local_normalizedyaw_3 45.0) (< _local_normalizedyaw_3 135.0))
      (return "NewEnumerator3")
      (elif (and (< _local_normalizedyaw -45.0) (> _local_normalizedyaw -135.0))
        (return "NewEnumerator4")
        (else
          (return "NewEnumerator2"))))))

(fn `RecieveDamage`
  (params (InHitResult :type "HitResult Structure") (InDamagingActor :type "Actor Object Reference"))
  (locals (Local_NormalizedYaw :type "Float (double-precision)"))
  (`self.ServerPlayHitAnimation` (`self.GetHitDirection` (`local.InDamagingActor`))))

(fn `SpawnMeleeEffects`
  (params (InImpactNormal :type "Vector Structure"))
  (bind (_returnvalue_x _returnvalue_y _returnvalue_z) (`KismetMathLibrary.BreakVector` (`Actor.K2_GetActorLocation` (`self.GetOwner`))))
  (`GameplayStatics.SpawnEmitterAtLocation` "/Game/CombatSystem/Art/SwordAnimsetPro/Demo/FX/Particles/P_HitPoint.P_HitPoint" (`KismetMathLibrary.MakeVector` _returnvalue_x _returnvalue_y (+ _returnvalue_z 25.0)) (`KismetMathLibrary.Conv_VectorToRotator` (`local.InImpactNormal`)))
  (`GameplayStatics.PlaySoundAtLocation` "/Game/CombatSystem/Art/Sound/Sword_Hit_05.Sword_Hit_05" (`Actor.K2_GetActorLocation` (`self.GetOwner`)) (struct) 0.07 1.0 0.0 null null null null))